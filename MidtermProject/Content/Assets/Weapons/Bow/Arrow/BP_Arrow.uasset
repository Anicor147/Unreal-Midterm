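; BP_Arrow is a bow arrow actor that damages Golden Knights and the Boss on contact.
; Its capsule overlap casts the other actor to each enemy type, calling OnHit on a knight or LooseHP on the boss, then destroys the arrow.
; A DoOnce on each branch guards against repeat hits, and an arrow that hits neither enemy destroys itself after a short delay from BeginPlay.
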(event OnComponentBeginOverlap(Capsule)
  (params (OverlappedComponent :type Primitive%20Component%20Object%20Reference) (OtherActor :type Actor%20Object%20Reference) (OtherComp :type Primitive%20Component%20Object%20Reference) (OtherBodyIndex :type Integer) (bFromSweep :type Boolean) (SweepResult :type Hit%20Result%20Structure%20%28by%20ref%29))
  (Utilities|FlowControl|Sequence
    (:then_0
      (Utilities|IsValid OtherActor
        (:Is%20Valid
          (bind _asbp_golden_knight (Utilities|Casting|CastToBP_GoldenKnight OtherActor))
          (Utilities|FlowControl|DoOnce false
            (:Completed
              (Default|OnHit _asbp_golden_knight 0.5)
              (Actor|DestroyActor))))))
    (:then_1
      (Utilities|IsValid OtherActor
        (:Is%20Valid
          (bind _asbp_boss (Utilities|Casting|CastToBP_Boss OtherActor))
          (Utilities|FlowControl|DoOnce false
            (:Completed
              (Default|LooseHP _asbp_boss)
              (Actor|DestroyActor))))))))

(event EventBeginPlay
  (Utilities|FlowControl|Delay 2.0)
  (Actor|DestroyActor))

(fn ConstructionScript)