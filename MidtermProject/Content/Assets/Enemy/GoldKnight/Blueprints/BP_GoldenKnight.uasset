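; BP_GoldenKnight is the Golden Knight enemy, handling its health, world-space health bar and death.
; BeginPlay passes itself to the WBP_GKHealthBar widget and hides it, while Tick rotates the bar to face the player camera.
; OnHit lowers Health and reveals the bar, with a delayed DoOnce reset throttling repeat hits.
; At zero health, a death montage plays once and its notify destroys the actor.
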(event Custom|RotateHealthBarToPlayer
  ;[0.01938 0.01938 0.01938] Rotate Widget to Player
  (Transformation|SetWorldRotation (Variables|Default|GetWidget) (Math|Rotator|CombineRotators (Camera|GetCameraRotation (Game|GetPlayerCameraManager 0)) "0.000000,180.000000,0.000000") false false))

(event Custom|SetReferenceToWidget
  ;[0.02732 0.02732 0.02732] Set Reference To Widget
  (bind _aswbp_gkhealth_bar (Utilities|Casting|CastToWBP_GKHealthBar (UserInterface|GetUserWidgetObject (Variables|Default|GetWidget))))
  (Variables|/Game/Assets/Enemy/GoldKnight/Blueprints/WBP_GKHealthBar.WBP_GKHealthBar_C|SetGKCharacter _aswbp_gkhealth_bar self))

(event Custom|OnHit
  ;[1 0.01317 0] On Hit Event
  (Utilities|FlowControl|DoOnce false :!label _label
    (:Completed
      (Variables|Default|SetHealth (- (Variables|Default|GetHealth) 0.2))
      (CallFunction|SetWidgetVisibilityHidden true)
      (CallFunction|OnDeath)
      (Utilities|FlowControl|Delay 0.5)
      (goto _label Reset))))

(event Custom|OnDeath
  ;[1 0.3499 0.3001] Play Death Animation
  (if (<= (Variables|Default|GetHealth) 0.0)
    (Utilities|FlowControl|DoOnce false
      (:Completed
        (Animation|Montage|PlayMontage (Variables|Default|GetSkeletalMesh) "/Game/Assets/Enemy/GoldKnight/Assets/Animations/AM_GoldenDead.AM_GoldenDead"
          (:OnNotifyBegin
            (Actor|DestroyActor self)))))))

(event EventBeginPlay
  (Utilities|FlowControl|Sequence
    (:then_0
      (CallFunction|SetReferencetoWidget))
    (:then_1
      (CallFunction|SetWidgetVisibilityHidden false))))

(event EventTick
  (params (DeltaSeconds :type Float%20%28single-precision%29))
  (CallFunction|RotateHealthBartoPlayer))

(fn ConstructionScript)

(fn SetWidgetVisibilityHidden
  (params (IsVisible :type Boolean))
  (bind _widget (Variables|Default|GetWidget))
  (bind _returnvalue (UserInterface|GetUserWidgetObject _widget))
  (if IsVisible
    (bind _output_get (LocalVariables|SetVisiblityState "Visible"))
    (Widget|SetVisibility _returnvalue _output_get)
    (else
      (bind _output_get_2 (LocalVariables|SetVisiblityState "Hidden"))
      (Widget|SetVisibility _returnvalue _output_get_2))))