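; AI controller for the Golden Knight enemy that runs its behavior tree and detects the player.
; On BeginPlay it starts BT_GK, caches the player and seeds the blackboard with the spawn position as patrol origin plus the knight's patrol location.
; Each tick, a line trace confirms sight of a player within a mid-distance band and sets TargetActor, which this controller never clears.
; It also draws a debug sphere at the inner radius and tracks a walking flag.
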(event EventBeginPlay
  (Utilities|FlowControl|Sequence
    (:then_0
      (Class|AIController|UseBlackboard "/Game/Assets/Enemy/GoldKnight/Blueprints/BB_GK.BB_GK")
      (AI|RunBehaviorTree "/Game/Assets/Enemy/GoldKnight/Blueprints/BT_GK.BT_GK")
      (bind _asbp_third_person_character (Utilities|Casting|CastToBP_ThirdPersonCharacter (Game|Player|GetPlayerPawn 0)))
      (Variables|Default|SetPlayer _asbp_third_person_character))
    (:then_1
      (AI|Components|Blackboard|SetValueasVector (AI|GetBlackboard 0) (Utilities|Name|MakeLiteralName "PatrolOrigin") (Transformation|GetActorLocation (Pawn|GetControlledPawn)))
      (bind _asbp_golden_knight (Utilities|Casting|CastToBP_GoldenKnight (Pawn|GetControlledPawn)))
      (AI|Components|Blackboard|SetValueasVector (AI|GetBlackboard 0) (Utilities|Name|MakeLiteralName "PatrolLocation") (Variables|/Game/Assets/Enemy/GoldKnight/Blueprints/BP_GoldenKnight.BP_GoldenKnight_C|GetPatrolLocation _asbp_golden_knight)))
    (:then_2
      (Variables|Default|SetisGKWalking true))))

(event EventTick
  (params (DeltaSeconds :type Float%20%28single-precision%29))
  (bind _returnvalue (Pawn|GetControlledPawn))
  (bind _returnvalue_2 (Pawn|GetControlledPawn))
  (bind _player (Variables|Default|GetPlayer))
  (bind _returnvalue_3 (Transformation|GetActorLocation _player))
  (bind _returnvalue_4 (Transformation|GetActorLocation _returnvalue))
  (bind _returnvalue_5 (Math|Vector|Distance(Vector) _returnvalue_4 _returnvalue_3))
  ;[1 0.06879 0] Check When Player is in Range
  (Utilities|IsValid _returnvalue
    (:Is%20Valid
      (Utilities|FlowControl|Sequence
        (:then_0
          (Rendering|Debug|DrawDebugSphere _returnvalue_4 5e+02 12 "(R=1.000000,G=1.000000,B=1.000000,A=1.000000)" 0.0))
        (:then_1
          (if (and (> _returnvalue_5 5e+02) (< _returnvalue_5 1e+03))
            (bind _outhit (Collision|LineTraceByChannel (Transformation|GetActorLocation _returnvalue_2) (Transformation|GetActorLocation (Variables|Default|GetPlayer)) "TraceTypeQuery2" false (Utilities|Array|MakeArray _returnvalue_2) "None"))
            (bind _asbp_third_person_character (Utilities|Casting|CastToBP_ThirdPersonCharacter (.hitactor _outhit)))
            (AI|Components|Blackboard|SetValueasObject (AI|GetBlackboard 0) (Utilities|Name|MakeLiteralName "TargetActor") _asbp_third_person_character)))))))

(fn ConstructionScript)

(fn CharacterIsWalking
  (params (CheckIsWalking :type Boolean))
  (Variables|Default|SetisGKWalking CheckIsWalking))