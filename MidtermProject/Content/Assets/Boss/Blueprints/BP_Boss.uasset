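; Boss character with melee and spell attacks, a phase-two flag, and death handling.
; On play it links itself to its health bar widget; LooseHP lowers HP, and death unpossesses the AI controller before a delayed destroy.
; Slash montage notifies toggle Capsule1 collision, whose overlap hits the player unless blocking.
; The spell montage spawns an energy ball at an arrow component, with DoOnce gates preventing attack re-triggering.
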(event OnComponentBeginOverlap(Capsule1)
  (params (OverlappedComponent :type Primitive%20Component%20Object%20Reference) (OtherActor :type Actor%20Object%20Reference) (OtherComp :type Primitive%20Component%20Object%20Reference) (OtherBodyIndex :type Integer) (bFromSweep :type Boolean) (SweepResult :type Hit%20Result%20Structure%20%28by%20ref%29))
  ;[1 0 0.118] Attack Player
  (bind _asbp_third_person_character (Utilities|Casting|CastToBP_ThirdPersonCharacter OtherActor))
  (if (not (Variables|/Game/Blueprints/Character/BP_ThirdPersonCharacter.BP_ThirdPersonCharacter_C|GetisPBlocking _asbp_third_person_character))
    (Default|PlayerIsHit _asbp_third_person_character)))

(event Custom|Phase2Condition
  ;[1 0.1085 0.5566] Phase2 Condition
  (if (<= (Variables|Default|GetHp) 1e+02)
    (Variables|Default|SetisPhase2 true)
    (else
      (Variables|Default|SetisPhase2 false))))

(event Custom|SetReferenceToWidget
  ;[0.1596 1 0] Set Reference to widget
  (bind _aswbp_boss_health_bar (Utilities|Casting|CastToWBP_BossHealthBar (UserInterface|GetUserWidgetObject (Variables|Default|GetWidget))))
  (Variables|/Game/Assets/Boss/Blueprints/WBP_BossHealthBar.WBP_BossHealthBar_C|SetBoss _aswbp_boss_health_bar self))

(event Custom|LooseHP
  ;[0 1 0.2199] Check HP
  (Utilities|FlowControl|Sequence
    (:then_0
      (Utilities|FlowControl|DoOnce false :!label _label
        (:Completed
          (if (not (<= (Variables|Default|GetHp) 0.0))
            (bind _output_get (Variables|Default|SetHp (- (Variables|Default|GetHp) 0.5)))
            (Development|PrintString (Utilities|String|ToString(Float) _output_get))
            (goto _label Reset)
            (else
              (CallFunction|OnDeath (Variables|Default|GetHp))
              (Utilities|FlowControl|Delay 0.5))))))
    (:then_1
      (if (<= (Variables|Default|GetHp) 0.5)
        (Variables|Default|SetisPhase2 true)))))

(event Custom|OnDeath
  (params (Health :type Float%20%28double-precision%29))
  (bind _self self)
  ;[0.05399 0 1] On Death
  (if (<= Health 0.0)
    (Variables|Default|SetisDead true)
    (Utilities|IsValid _self
      (:Is%20Valid
        (Utilities|FlowControl|DoOnce false
          (:Completed
            (Pawn|UnPossess (AI|GetAIController _self))
            (Utilities|FlowControl|Delay 5.0)
            (Actor|DestroyActor self)))))))

(event Custom|BossAttackAnim
  ;[1 0 0.7633] Play Attack Animation
  (Utilities|FlowControl|DoOnce false :!label _label
    (:Completed
      (bind _notifyname (Animation|Montage|PlayMontage (Variables|Character|GetMesh) "/Game/Assets/Boss/Animation/AM_Slash.AM_Slash")
        (:OnCompleted
          (goto _label Reset))
        (:OnNotifyBegin
          (switch name _notifyname
            (:Start
              (Collision|SetCollisionEnabled (Variables|Default|GetCapsule1) "QueryAndPhysics"))
            (:End
              (Collision|SetCollisionEnabled (Variables|Default|GetCapsule1) "NoCollision"))))))))

(event Custom|SpellAttack
  ;[1 1 1] SpawnEnergy
  (Utilities|FlowControl|DoOnce false :!label _label
    (:Completed
      (Animation|Montage|PlayMontage (Variables|Character|GetMesh) "/Game/Assets/Boss/Animation/AM_SpellAttack.AM_SpellAttack"
        (:OnNotifyBegin
          (Game|SpawnActorfromClass "/Game/Assets/Boss/Blueprints/BP_EnergyBall.BP_EnergyBall_C" (Transformation|GetWorldTransform (Variables|Default|GetArrow1)) "Undefined" "MultiplyWithRoot" 0 0)
          (Utilities|FlowControl|Delay 1.0)
          (goto _label Reset))))))

(event EventBeginPlay
  ;[1 0.005162 0] Begin Play
  (Utilities|FlowControl|Sequence
    (:then_0
      (CallFunction|SetReferencetoWidget))
    (:then_1
      (CallFunction|SetWidgetVisibilityHidden true))))

(fn ConstructionScript)

(fn SetWidgetVisibilityHidden
  (params (IsVisible :type Boolean)))