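; AI controller for the boss that runs its behavior tree and feeds the blackboard with player detection and phase state.
; BeginPlay caches the player and stores the pawn's starting location as Origin.
; Tick sets CanSeePlayer by distance alone, while an in-range visibility trace hitting the player sets TargetActor, with debug drawing enabled.
; Tick also flags Phase2 when BP_Boss health falls to half or below.
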(event EventBeginPlay
  (bind _returnvalue (Pawn|GetControlledPawn))
  (Utilities|FlowControl|Sequence
    (:then_0
      (Class|AIController|UseBlackboard "/Game/Assets/Boss/Blueprints/BB_Boss.BB_Boss")
      (AI|RunBehaviorTree "/Game/Assets/Boss/Blueprints/BTT_Boss.BTT_Boss")
      (bind _asbp_third_person_character (Utilities|Casting|CastToBP_ThirdPersonCharacter (Game|Player|GetPlayerPawn 0)))
      (Variables|Default|SetPlayer _asbp_third_person_character))
    (:then_1
      (Utilities|IsValid _returnvalue
        (:Is%20Valid
          (AI|Components|Blackboard|SetValueasVector (AI|GetBlackboard 0) (Utilities|Name|MakeLiteralName "Origin") (Transformation|GetActorLocation _returnvalue)))))
    (:then_3
      (Utilities|Casting|CastToBP_GoldenKnight (Pawn|GetControlledPawn))
      (AI|Components|Blackboard|SetValueasBool (AI|GetBlackboard 0) (Utilities|Name|MakeLiteralName "CanSeePlayer") false))))

(event EventTick
  (params (DeltaSeconds :type Float%20%28single-precision%29))
  (bind _returnvalue (Pawn|GetControlledPawn))
  (bind _returnvalue_2 (Pawn|GetControlledPawn))
  (bind _returnvalue_3 (Transformation|GetActorLocation _returnvalue_2))
  ;[1 0.06879 0] Check When Player is in Range
  (Utilities|IsValid _returnvalue_2
    (:Is%20Valid
      (Utilities|FlowControl|Sequence
        (:then_0
          (Rendering|Debug|DrawDebugSphere _returnvalue_3 3e+03 12 "(R=1.000000,G=1.000000,B=1.000000,A=1.000000)" 0.0))
        (:then_1
          (if (< (Math|Vector|Distance(Vector) _returnvalue_3 (Transformation|GetActorLocation (Variables|Default|GetPlayer))) 3e+03)
            (AI|Components|Blackboard|SetValueasBool (AI|GetBlackboard 0) (Utilities|Name|MakeLiteralName "CanSeePlayer") true)
            (bind _outhit (Collision|LineTraceByChannel (Transformation|GetActorLocation _returnvalue) (Transformation|GetActorLocation (Variables|Default|GetPlayer)) "TraceTypeQuery1" false (Utilities|Array|MakeArray _returnvalue) "Persistent"))
            (bind _asbp_third_person_character (Utilities|Casting|CastToBP_ThirdPersonCharacter (.HitActor (Collision|BreakHitResult _outhit))))
            (AI|Components|Blackboard|SetValueasObject (AI|GetBlackboard 0) (Utilities|Name|MakeLiteralName "TargetActor") _asbp_third_person_character)
            (else
              (AI|Components|Blackboard|SetValueasBool (AI|GetBlackboard 0) (Utilities|Name|MakeLiteralName "CanSeePlayer") false))))
        (:then_2
          (bind _asbp_boss (Utilities|Casting|CastToBP_Boss (Pawn|GetControlledPawn)))
          (if (<= (Variables|/Game/Assets/Boss/Blueprints/BP_Boss.BP_Boss_C|GetHp _asbp_boss) 0.5)
            (AI|Components|Blackboard|SetValueasBool (AI|GetBlackboard 0) (Utilities|Name|MakeLiteralName "Phase2") true)))))))

(fn ConstructionScript)