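; BP_GameState tracks a lantern-ordering puzzle, checking each reported lantern value against the LanternSequence array.
; A correct value advances Index and prints a success message once Index equals the value stored in the array's last element, rather than its length.
; A wrong value resets Index, spawns a BP_GoldenKnight at the supplied position and hides the fire on every BP_InteractionLantern.
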(event Custom|LanternSequenceEvent
  (params (LanternValue :type Integer) (Position :type Vector))
  (bind _lanternsequence (Variables|Default|GetLanternSequence))
  (if (== LanternValue (Utilities|Array|Get(acopy) (Variables|Default|GetLanternSequence) (Variables|Default|Getindex)))
    (Math|Integer|IncrementInt (Variables|Default|Getindex)
      (:%20%20
        (if (== (Variables|Default|Getindex) (Utilities|Array|Get(acopy) _lanternsequence (Utilities|Array|LastIndex _lanternsequence)))
          (Development|PrintString "Gut job"))))
    (else
      (Variables|Default|Setindex 0)
      (Game|SpawnActorfromClass "/Game/Assets/Enemy/GoldKnight/Blueprints/BP_GoldenKnight.BP_GoldenKnight_C" (Math|Transform|MakeTransform Position "0, 0, 0" "1.000000,1.000000,1.000000") "AlwaysSpawn" "MultiplyWithRoot" 0 0)
      (bind _outactors (Actor|GetAllActorsOfClass "/Game/Blueprints/Interaction/BP_InteractionLantern.BP_InteractionLantern_C"))
      (for _array_element _outactors
        (bind _asbp_interaction_lantern (Utilities|Casting|CastToBP_InteractionLantern _array_element))
        (Rendering|SetVisibility (Variables|/Game/Blueprints/Interaction/BP_InteractionLantern.BP_InteractionLantern_C|GetP_Fire _asbp_interaction_lantern) false false)))))

(fn ConstructionScript)