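; Base Blueprint for interactable objects, with a Widget that can be shown or hidden.
; The Widget is hidden on BeginPlay, and the Show and Hide events toggle its visibility without propagating to child components.
; The OnInteraction function only prints a message with the object's display name.
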(event Custom|Hide
  (Rendering|SetVisibility (Variables|Default|GetWidget) false false))

(event Custom|Show
  (Rendering|SetVisibility (Variables|Default|GetWidget) true false))

(event EventBeginPlay
  (CallFunction|Hide))

(fn ConstructionScript)

(fn OnInteraction
  (Development|PrintString (Utilities|String|Append "You interacted with : " (Utilities|GetDisplayName self))))